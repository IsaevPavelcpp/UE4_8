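; Block grid actor for a ball-and-blocks game, where blocks react to hits from BP_ball.
; The construction script lays out static mesh components in an X by Y grid spaced by Padding.
; On a hit, a material comparison helper feeds ColorOrDeath, which either turns that block red or destroys it and spawns a BP_baseBonus at a fixed location.
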(event EventBeginPlay)

(event Collision|EventActorBeginOverlap
  (params (OtherActor :type Actor%20Object%20Reference)))

(event EventTick
  (params (DeltaSeconds :type Float%20%28single-precision%29)))

(event Collision|EventHit
  (params (MyComp :type Primitive%20Component%20Object%20Reference) (Other :type Actor%20Object%20Reference) (OtherComp :type Primitive%20Component%20Object%20Reference) (bSelfMoved :type Boolean) (HitLocation :type Vector :default "0, 0, 0") (HitNormal :type Vector :default "0, 0, 0") (NormalImpulse :type Vector :default "0, 0, 0") (Hit :type Hit%20Result%20Structure%20%28by%20ref%29))
  (Utilities|Casting|CastToBP_ball Other)
  (CallFunction|ColororDeath MyComp MyComp (|comparisonofthematerial MyComp)))

(fn ConstructionScript
  (for _index (range 1 (Variables|Default|GetY))
    (for _index_2 (range 1 (Variables|Default|GetX))
      (AddComponent|AddStaticMeshComponent false (Math|Transform|MakeTransform (Math|Vector|MakeVector (Math|Conversions|ToFloat(Integer) (* _index_2 (Variables|Default|Getpadding))) (Math|Conversions|ToFloat(Integer) (* _index (Variables|Default|Getpadding))) 0.0))))))

(fn ColororDeath
  (params (self2 :type Primitive%20Component%20Object%20Reference) (self3 :type Actor%20Component%20Object%20Reference) (Condition :type Boolean))
  (if Condition
    (Components|DestroyComponent self3)
    (bind _returnvalue (Game|SpawnActorfromClass "/Game/Blueprints/Construction/BP_baseBonus.BP_baseBonus_C" (Math|Transform|MakeTransform "10.000000,-50.000000,50.000000") "AlwaysSpawn" 0 0))
    (Variables|Default|SetBP_bonus _returnvalue)
    (return)
    (else
      (Rendering|Material|SetMaterial self2 0 "/AnimationSharing/AnimSharingRed.AnimSharingRed"))))