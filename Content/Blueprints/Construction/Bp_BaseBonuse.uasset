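; Base bonus pickup that grants a random effect to BP_Pown when a Hit event involves it.
; Weighted random picks a less likely extra ball (BP_ballBonus), an added life, or a temporary X-axis widening.
; Ball and life bonuses destroy the pickup immediately.
; The size bonus swaps the sphere material and disables collision, then reverts the scale after a delay without destroying the pickup.
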(event EventBeginPlay
  (Variables|Default|Setspeed 5.0)
  (Variables|Default|Setdirection "0,-90.000000, 0"))

(event Collision|EventActorBeginOverlap
  (params (OtherActor :type Actor%20Object%20Reference)))

(event Collision|EventHit
  (params (MyComp :type Primitive%20Component%20Object%20Reference) (Other :type Actor%20Object%20Reference) (OtherComp :type Primitive%20Component%20Object%20Reference) (bSelfMoved :type Boolean) (HitLocation :type Vector :default "0, 0, 0") (HitNormal :type Vector :default "0, 0, 0") (NormalImpulse :type Vector :default "0, 0, 0") (Hit :type Hit%20Result%20Structure%20%28by%20ref%29))
  (bind _asbp_pown (Utilities|Casting|CastToBP_Pown Other))
  (if (Math|Random|RandomBoolwithWeight 0.2)
    (|bonusBall _asbp_pown)
    (elif (Math|Random|RandomBoolwithWeight 0.5)
      (|bonusSize _asbp_pown _asbp_pown _asbp_pown)
      (else
        (|bonusLive _asbp_pown)))))

(fn ConstructionScript
  (|CallParentFunction))