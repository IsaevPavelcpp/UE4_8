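; BP_ballBonus is a bonus ball actor that bounces around the level until it falls into a kill volume.
; Each tick it moves along Direction at Speed with a swept world offset, and a blocking hit replaces Direction with a reflection computed from the surface normal's X and Y.
; Overlapping a KillZVolume prints a debug message and destroys the ball.
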(event Collision|EventActorBeginOverlap
  (params (OtherActor :type Actor%20Object%20Reference))
  (Utilities|Casting|CastToKillZVolume OtherActor)
  (Development|PrintString "bonusBallFall" true true "(R=0.288183,G=1.000000,B=0.000000,A=1.000000)")
  (Actor|DestroyActor))

(event EventTick
  (params (DeltaSeconds :type Float%20%28single-precision%29))
  (bind _sweephitresult (Transformation|AddActorWorldOffset (* (* (Variables|Default|Getdirection) (Variables|Default|Getspeed)) DeltaSeconds) true))
  (if (.bBlockingHit (Collision|BreakHitResult _sweephitresult))
    (Variables|Default|SetDirection (Math|Vector|GetReflectionVector (Variables|Default|GetDirection) (Math|Vector|MakeVector (.X (Math|Vector|BreakVector (.Normal (Collision|BreakHitResult _sweephitresult)))) (.Y (Math|Vector|BreakVector (.Normal (Collision|BreakHitResult _sweephitresult)))) 0.0)))))

(fn ConstructionScript)