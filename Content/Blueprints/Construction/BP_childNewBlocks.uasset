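; Construction Blueprint that lays out a flat grid of child actors, apparently blocks, in the editor.
; The construction script calls its parent, then nested loops over Y and X add a Child Actor Component per cell, offset in X and Y by index times Padding.
; The event graph holds only disabled default events, so it adds no runtime logic.
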(event EventBeginPlay
  (|CallParentFunction) ; This node is disabled and will not be called.\nDrag off pins to build functionality.
)

(event Collision|EventActorBeginOverlap
  (params (OtherActor :type Actor%20Object%20Reference))
  (|CallParentFunction OtherActor) ; This node is disabled and will not be called.\nDrag off pins to build functionality.
)

(event EventTick
  (params (DeltaSeconds :type Float%20%28single-precision%29))
  (|CallParentFunction DeltaSeconds) ; This node is disabled and will not be called.\nDrag off pins to build functionality.
)

(fn ConstructionScript
  (|CallParentFunction)
  (for _index (range 1 (Variables|Default|Gety))
    (for _index_2 (range 1 (Variables|Default|Getx))
      (AddComponent|AddChildActorComponent false (Math|Transform|MakeTransform (Math|Vector|MakeVector (Math|Conversions|ToFloat(Integer) (* _index_2 (Variables|Default|Getpadding))) (Math|Conversions|ToFloat(Integer) (* _index (Variables|Default|Getpadding))) 0.0))))))